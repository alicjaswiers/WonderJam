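; Game state Blueprint that runs the in-game day clock for the BP_CustomSkySun actor.
; On BeginPlay it finds that actor, converts its starting time to total seconds and starts a looping timer.
; Each tick adds a configurable number of game seconds, scaling game time against real time, and writes hours, minutes and seconds back to the sun actor.
; The counter resets to zero once it reaches a full day.
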(event `self.ReceiveBeginPlay`
  (bind _returnvalue (`GameplayStatics.GetActorOfClass` "/Game/Art/Sky/Environment/BP_CustomSkySun.BP_CustomSkySun_C"))
  (bind _output_get (set `self.SkySun` _returnvalue))
  (set `self.TimeInSeconds` (`KismetMathLibrary.FTrunc` (`KismetMathLibrary.GetTotalSeconds` (`KismetMathLibrary.MakeTimespan` 0 (`/Game/Art/Sky/Environment/BP_CustomSkySun.Hours` _output_get) (`/Game/Art/Sky/Environment/BP_CustomSkySun.Minutes` _output_get) (`/Game/Art/Sky/Environment/BP_CustomSkySun.Seconds` _output_get)))))
  (`KismetSystemLibrary.K2_SetTimerDelegate` (delegate `TimeUpdate`) (/ 1.0 (`self.AmountToTickSec`)) true))

(event `TimeUpdate`
  (bind _skysun (`self.SkySun`))
  (bind _output_get (set `self.TimeInSeconds` (+ (`self.TimeInSeconds`) (`self.AmountOfSecToAddPerTick`))))
  (bind (_days _hours _minutes _seconds) (`KismetMathLibrary.BreakTimespan` (`KismetMathLibrary.MakeTimespan` 0 0 0 _output_get)))
  (set `/Game/Art/Sky/Environment/BP_CustomSkySun.Hours` _hours _skysun)
  (set `/Game/Art/Sky/Environment/BP_CustomSkySun.Minutes` _minutes _skysun)
  (set `/Game/Art/Sky/Environment/BP_CustomSkySun.Seconds` _seconds _skysun)
  (if (>= (`self.TimeInSeconds`) 86400)
    (set `self.TimeInSeconds` 0)))

(fn `UserConstructionScript`)