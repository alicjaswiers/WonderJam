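; BP_DamageManager is a helper actor providing damage feedback, death handling and enemy health bar updates.
; Hurt and Death play a given sound and spawn an effect at the target's location, with Death also destroying it.
; Health bar functions cast widgets to WB_EnemyHealthBar to set full HP, blacken the fill or apply damage.
; UpdateHealthBar returns clamped new health and a normalized HP that never drops below a quarter.
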(fn `Death`
  (params (Sound :type "SoundBase Object Reference") (Effect :type "NiagaraSystem Object Reference") (Actor :type "Actor Object Reference"))
  (bind _returnvalue (`self.K2_GetActorLocation` Actor))
  ;[1 1 1] Death
  (`GameplayStatics.PlaySoundAtLocation` Sound _returnvalue (struct) 1.0 1.0 0.0 null null null null)
  (`NiagaraFunctionLibrary.SpawnSystemAtLocation` Effect _returnvalue)
  (`self.K2_DestroyActor` Actor))

(fn `Hurt`
  (params (Sound :type "SoundBase Object Reference") (Effect :type "NiagaraSystem Object Reference") (Actor :type "Actor Object Reference"))
  (bind _returnvalue (`self.K2_GetActorLocation` Actor))
  (`GameplayStatics.PlaySoundAtLocation` Sound _returnvalue (struct) 1.0 1.0 0.0 null null null null)
  (`NiagaraFunctionLibrary.SpawnSystemAtLocation` Effect _returnvalue))

(fn `SetHealthBar`
  (params (Health :type "Float (double-precision)") (HealthBar :type "WidgetComponent Object Reference"))
  (bind _aswb_enemy_health_bar (cast `/Game/UI/WB_EnemyHealthBar` (`WidgetComponent.GetUserWidgetObject` HealthBar)))
  (set `/Game/UI/WB_EnemyHealthBar.HP%` (/ Health Health) _aswb_enemy_health_bar))

(fn `SetHealthbarLook`
  (params (HealthBar :type "WidgetComponent Object Reference"))
  (bind _aswb_enemy_health_bar (cast `/Game/UI/WB_EnemyHealthBar` (`WidgetComponent.GetWidget` HealthBar)))
  (`ProgressBar.SetFillColorAndOpacity` (`/Game/UI/WB_EnemyHealthBar.ProgressBar` _aswb_enemy_health_bar) (struct :`A` 1.0)))

(fn `Update Health Bar`
  (params (Health :type "Float (double-precision)") (Damage :type "Float (double-precision)") (MaxHealth :type "Float (double-precision)") (HealthBar :type "WidgetComponent Object Reference"))
  (returns (`HP%` :type "Float (double-precision)") (NewHealth :type "Float (double-precision)"))
  (bind _returnvalue (`KismetMathLibrary.FClamp` (- Health Damage) 0.0 MaxHealth))
  (bind _aswb_enemy_health_bar (cast `/Game/UI/WB_EnemyHealthBar` (`WidgetComponent.GetWidget` HealthBar)))
  (bind _output_get (set `/Game/UI/WB_EnemyHealthBar.HP%` (`KismetMathLibrary.FClamp` (/ _returnvalue MaxHealth) 0.25) _aswb_enemy_health_bar))
  (return _output_get _returnvalue))

(fn `UserConstructionScript`)