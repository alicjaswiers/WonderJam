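; BP_FlowerNPC is a targetable flower NPC that pleads for its life while a tutorial prompts the player to kill it.
; Tick turns its mesh on yaw only to face the player.
; BeginPlay sets up the health bar, then uses delays to show the plea with a sound and add the tutorial widget.
; The Kill event shows a scream, waits briefly, destroys the actor and spawns an explosion.
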(event `self.ReceiveTick`
  (params (DeltaSeconds :type "Float (single-precision)"))
  (bind _mesh (`self.Mesh`))
  ;[1 1 1] Set Aim rotation
  (`SceneComponent.K2_SetWorldRotation` _mesh (`KismetMathLibrary.MakeRotator` 0.0 0.0 (+ (.yaw (`KismetMathLibrary.FindLookAtRotation` (`SceneComponent.K2_GetComponentLocation` _mesh) (`self.K2_GetActorLocation` (`GameplayStatics.GetPlayerCharacter` 0)))) -100.0)) false false))

(event `self.ReceiveBeginPlay`
  (bind _aswb_enemy_health_bar (cast `/Game/UI/WB_EnemyHealthBar` (`WidgetComponent.GetUserWidgetObject` (`self.HealthBar`))))
  (`ProgressBar.SetFillColorAndOpacity` (`/Game/UI/WB_EnemyHealthBar.ProgressBar` _aswb_enemy_health_bar) (struct :`A` 1.0))
  (set `/Game/UI/WB_EnemyHealthBar.HP%` 0.25 _aswb_enemy_health_bar)
  (bind _aswb_text (cast `/Game/UI/WB_Text` (`WidgetComponent.GetUserWidgetObject` (`self.Text`))))
  (set `self.As WB Text` _aswb_text)
  (`KismetSystemLibrary.Delay` 2.0)
  (set `/Game/UI/WB_Text.Text` "Please don't kill me" (`self.As WB Text`))
  (`GameplayStatics.PlaySoundAtLocation` "/Engine/VREditor/Sounds/UI/Camera_Shutter.Camera_Shutter" (`self.K2_GetActorLocation`) (struct) 1.0 1.0 0.0 null null null null)
  (`KismetSystemLibrary.Delay` 1.0)
  (bind _returnvalue (`|CreateWidget` "/Game/UI/WB_Tutorials.WB_Tutorials_C"))
  (`UserWidget.AddToViewport` _returnvalue 0)
  (set `/Game/UI/WB_Tutorials.Text` "Press left mouse to kill flower hehe" _returnvalue))

(event `/Game/HealthSystem/BP_Kill.Kill`
  ;[1 1 1] Kill npc
  (set `/Game/UI/WB_Text.Text` "NOOOO" (`self.As WB Text`))
  (`KismetSystemLibrary.Delay` 1.0)
  (`self.K2_DestroyActor`)
  (`GameplayStatics.SpawnEmitterAtLocation` "/Game/StarterContent/Particles/P_Explosion.P_Explosion" (`self.K2_GetActorLocation`) (struct) (2.0 2.0 2.0)))

(fn `IsTargettable`
  (returns (IsTargettable :type Boolean))
  (return true))

(fn `UserConstructionScript`)