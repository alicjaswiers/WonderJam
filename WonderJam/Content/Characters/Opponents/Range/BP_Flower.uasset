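; BP_Flower is a ranged opponent pawn that the player can target, with stats, sounds and effects read from data tables by Name.
; Pawn sensing and a per-tick distance check feed the PlayerSeen and InRange blackboard keys.
; Damage updates health through the game mode's DamageManager; a bar value of exactly 0.25 makes it killable and unable to attack.
; Kill then triggers death and removes the player's targeting marker.
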(event `self.ReceiveTick`
  (params (DeltaSeconds :type "Float (single-precision)"))
  (bind _returnvalue (`AIBlueprintHelperLibrary.GetBlackboard` (`AIBlueprintHelperLibrary.GetAIController` self)))
  (bind _returnvalue_2 (`|GetDataTableRow` "/Game/HealthSystem/DT_Attack.DT_Attack" (`self.Name`))
    (:`then`
      ;[1 1 1] Get distance and check if in range
      (if (> (`self.GetDistanceTo` (`GameplayStatics.GetPlayerPawn` 0)) (`.AttackRange_13_6E1458394259B5D68CB914ACF56E37DA` (break `/Game/HealthSystem/AttackStats` _returnvalue_2)))
        ;[1 1 1] Set in range bool
        (`BlackboardComponent.SetValueAsBool` _returnvalue "InRange" false)
        (else
          (`BlackboardComponent.SetValueAsBool` _returnvalue "InRange" true))))))

(event `self.PawnSensing.OnSeePawn`
  (params (Pawn :type "Pawn Object Reference"))
  ;[1 1 1] Check if player seen
  (if (`self.IsPlayerControlled` Pawn)
    (`BlackboardComponent.SetValueAsBool` (`AIBlueprintHelperLibrary.GetBlackboard` (`AIBlueprintHelperLibrary.GetAIController` self)) "PlayerSeen" true)))

(event `/Game/HealthSystem/BP_Kill.Kill`
  ;[1 1 1] If killable, kill
  (if (`self.Killable`)
    (bind (_hp _hurtsound _hurteffect _deathsound _deatheffect) (break `/Game/HealthSystem/CharacterStats` (stale `self.ReceiveAnyDamage` _returnvalue)))
    (`/Game/HealthSystem/BP_DamageManager.Death` (`self.Damage Manager`) _deathsound _deatheffect self)
    ;[1 1 1] if it's target kill this object
    (bind _ashero_player_controller (cast `/Game/GameMods/HeroPlayerController` (`GameplayStatics.GetPlayerController` 0)))
    (if (== (`/Game/GameMods/HeroPlayerController.CurrentTarget` _ashero_player_controller) self)
      (`self.K2_DestroyActor` (`/Game/GameMods/HeroPlayerController.TargetterActorRef` _ashero_player_controller)))))

(event `self.ReceiveAnyDamage`
  (params (Damage :type "Float (single-precision)") (DamageType :type "DamageType Object Reference") (InstigatedBy :type "Controller Object Reference") (DamageCauser :type "Actor Object Reference"))
  (bind _damage_manager (`self.Damage Manager`))
  ;[1 1 1] Take data from data base
  (bind _returnvalue (`|GetDataTableRow` "/Game/HealthSystem/DT_Character.DT_Character" (`self.Name`))
    (:`then`
      (bind (_hp _hurtsound _hurteffect _deathsound _deatheffect) (break `/Game/HealthSystem/CharacterStats` _returnvalue))
      ;[1 1 1] Change HP
      (bind (_hp_ _newhealth) (`/Game/HealthSystem/BP_DamageManager.Update Health Bar` (`self.Damage Manager`) (`self.Health`) Damage _hp (`self.HealthBar`)))
      (set `self.Health` _newhealth)
      ;[1 1 1] Check if deadable
      (if (== _hp_ 0.25)
        (`/Game/HealthSystem/BP_DamageManager.SetHealthbarLook` _damage_manager (`self.HealthBar`))
        (set `self.Killable` true)
        (else
          (`/Game/HealthSystem/BP_DamageManager.Hurt` _damage_manager _hurtsound _hurteffect self))))))

(event `self.ReceiveBeginPlay`
  ;[1 1 1] Set game manager
  (bind _ashero_game_mode (cast `/Game/GameMods/HeroGameMode` (`GameplayStatics.GetGameMode`)))
  (set `self.Damage Manager` (`/Game/GameMods/HeroGameMode.Damage Manager` _ashero_game_mode))
  ;[1 1 1] Set HP
  (bind _returnvalue (`|GetDataTableRow` "/Game/HealthSystem/DT_Character.DT_Character" (`self.Name`))
    (:`then`
      (bind _output_get (set `self.Health` (`.HP_14_AC0C00F14BF35971F74E61916F42B0A7` (break `/Game/HealthSystem/CharacterStats` _returnvalue))))
      (`/Game/HealthSystem/BP_DamageManager.SetHealthBar` (`self.Damage Manager`) _output_get (`self.HealthBar`))
      (`BlackboardComponent.SetValueAsName` (`AIBlueprintHelperLibrary.GetBlackboard` (`AIBlueprintHelperLibrary.GetAIController` self)) "Name" (`self.Name`)))))

(fn `CanAttackFlower`
  (returns (CanAttack :type Boolean))
  (if (`self.Killable`)
    (return false)
    (else
      (return true))))

(fn `IsTargettable`
  (returns (IsTargettable :type Boolean))
  (return true))

(fn `UserConstructionScript`)